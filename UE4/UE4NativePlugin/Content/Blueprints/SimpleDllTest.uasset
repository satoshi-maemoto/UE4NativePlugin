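; SimpleDllTest is a test Blueprint that loads an external native DLL at runtime and calls a string function from it.
; BeginPlay imports SimpleDll.dll from the SimpleDll folder, then imports its GetStringValue method, with success and failure messages printed for both steps.
; Tick calls GetStringValue with a fixed argument and prints the result every frame, without checking that the import worked.
; EndPlay frees the DLL.
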(event `self.ReceiveBeginPlay`
  (`SimpleDllAccessor.importDLL` "SimpleDll" "SimpleDll.dll")
  (if true
    (`KismetSystemLibrary.PrintString` "DLL Import Sucess.")
    (`SimpleDllAccessor.importMethodGetStringValue`)
    (if true
      (`KismetSystemLibrary.PrintString` "Method Import Sucess")
      (else
        (`KismetSystemLibrary.PrintString` "Method Import Fail")))
    (else
      (`KismetSystemLibrary.PrintString` "DLL Import Fail."))))

(event `self.ReceiveTick`
  (params (DeltaSeconds :type "Float (single-precision)"))
  (bind _returnvalue (`SimpleDllAccessor.GetStringValue` 10))
  (`KismetSystemLibrary.PrintString` _returnvalue))

(event `self.ReceiveEndPlay`
  (params (EndPlayReason :type "EEndPlayReason Enum" :default "Destroyed"))
  (`SimpleDllAccessor.freeDLL`))

(fn `UserConstructionScript`)